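; BP_TheRobot is the playable robot character with a gun, chargeable grenade throw and backpack-deployed drone.
; On BeginPlay the player-controlled instance creates crosshair and grenade-charge widgets; aiming resizes the crosshair.
; Timelines drive arm recoil, movement-gated FOV changes, backpack doors and grenade charge.
; Timeline completions and Delays sequence drone launch and possession, then docking, robot repossession and crosshair re-creation.
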(event `self.ReceiveBeginPlay`
  (if (== (`GameplayStatics.GetPlayerPawn` 0) self)
    (bind _returnvalue (`|CreateWidget` "/Game/Blueprints/Widgets/Crosshair.Crosshair_C"))
    (`UserWidget.AddToViewport` _returnvalue 0)
    (set `self.CrosshairRef` _returnvalue)
    (bind _returnvalue_2 (`|CreateWidget` "/Game/Blueprints/Widgets/GrenadeMultiplier.GrenadeMultiplier_C"))
    (`UserWidget.AddToViewport` _returnvalue_2 0)
    (bind _output_get (set `self.WidgetGrenadeMultiplier` _returnvalue_2))
    (set `/Game/Blueprints/Widgets/GrenadeMultiplier.RobotRef` self _output_get))
  (set `self.BackpackBase` (`self.BP_BackpackBase`))
  (set `self.BackpackLeftDoor` (`self.Backpack_LeftDoor`))
  (set `self.BackpackRightDoor` (`self.BackPack_RightDoor`))
  (set `self.GunRef` (`self.Gun`)))

(event `self.ReceiveTick`
  (params (DeltaSeconds :type "Float (single-precision)")))

(event `self.StartAiming`
  (set `self.bIsAiming` true)
  (set `self.c_bIsAiming` true)
  (`/Game/Blueprints/Widgets/Crosshair.ShrinkCrosshair_F` (`self.CrosshairRef`)))

(event `self.StopAiming`
  (set `self.bIsAiming` false)
  (set `self.c_bIsAiming` false)
  (`/Game/Blueprints/Widgets/Crosshair.GrowCrosshair_F` (`self.CrosshairRef`)))

(event `self.PlayMuzzleEffect`
  (`ActorComponent.Activate` (`self.MuzzleEffect`) false))

(event `self.JoltArms`
  (bind (_direction _newtrack_0) (`Timeline|JoltTimeline` :!via `PlayFromStart`)
    (:`Update`
      (`SceneComponent.K2_SetRelativeLocation` (`self.Arms`) (`KismetMathLibrary.VLerp` (-2.211937 0.907197 -160.604034) (-5.873283 0.907334 -160.604034) _newtrack_0) false false))))

(event `self.IncreaseFOV`
  (`/Engine/EditorBlueprintResources/StandardMacros.CompareFloat` (`KismetMathLibrary.VSize` (`MovementComponent.Velocity` (`self.GetMovementComponent`)))
    (:`>`
      (`|ExecutionSequence`
        (:`then_0`
          (bind (_direction _newtrack_0) (`Timeline|TL_IncreaseFOV` :!via `Stop` :!label _label)
            (:`Update`
              (set `CameraComponent.FieldOfView` _newtrack_0 (`self.RobotCamera`)))))
        (:`then_1`
          (goto _label :!via `PlayFromStart`))))))

(event `self.DecreaseFOV`
  (`/Engine/EditorBlueprintResources/StandardMacros.CompareFloat` (`CameraComponent.FieldOfView` (`self.RobotCamera`)) 90.0
    (:`<`
      (`|ExecutionSequence`
        (:`then_0`
          (goto _label :!via `Stop`))
        (:`then_1`
          (goto _label :!via `Reverse`))))))

(event `self.OpenBackpack`
  (bind _spawneddrone (`self.SpawnedDrone`))
  (set `self.bJustOpenedBackpack` true)
  (bind (_direction _newtrack_0) (`Timeline|OpenBackpackTL` :`NewTime` 0.3 :!via `PlayFromStart` :!label _label_2)
    (:`Update`
      (`SceneComponent.K2_SetRelativeRotation` (`self.Backpack_LeftDoor`) (`KismetMathLibrary.RLerp` (`self.LeftDoorClosed`) (`self.LeftDoorOpen`) _newtrack_0 true) false false)
      (`SceneComponent.K2_SetRelativeRotation` (`self.BackPack_RightDoor`) (`KismetMathLibrary.RLerp` (`self.RightDoorClosed`) (`self.RightDoorOpen`) _newtrack_0 true) false false))
    (:`Finished`
      (if (`self.bJustOpenedBackpack`)
        (set `self.bJustOpenedBackpack` false)
        (`Widget.RemoveFromParent` (`self.CrosshairRef`))
        (`DroneCharacter.CallLiftFromBackPack` _spawneddrone)
        (`KismetSystemLibrary.Delay` 0.5)
        (`DroneCharacter.CallRotateToDeployed` _spawneddrone)
        (`KismetSystemLibrary.Delay` 0.4)
        (`self.PossessDrone`)))))

(event `self.CloseBackpack`
  (goto _label_2 :!via `Reverse`))

(event `self.PlaceDroneInBag`
  (bind _spawneddrone (`self.SpawnedDrone`))
  (bind (_direction _newtrack_0) (`Timeline|PlaceDroneAboveBackpack` :!via `PlayFromStart`)
    (:`Update`
      (`self.LerpDroneAboveBackPack` _newtrack_0))
    (:`Finished`
      (`DroneCharacter.CallRotateToBackPack` _spawneddrone)
      (`self.K2_AttachToActor` _spawneddrone self "BackpackLocation" "KeepWorld" "SnapToTarget" "KeepWorld" true)
      (`KismetSystemLibrary.Delay` 0.5)
      (`self.CloseBackpack`)
      (`KismetSystemLibrary.Delay` 0.6)
      (`self.RepossessRobot`)
      (bind _returnvalue (`|CreateWidget` "/Game/Blueprints/Widgets/Crosshair.Crosshair_C"))
      (bind _output_get (set `self.CrosshairRef` _returnvalue))
      (`UserWidget.AddToViewport` _output_get 0))))

(event `self.BuildUpGrenadeVelocity`
  (set `self.GrenadeMultiplier` 0.0)
  (`/Game/Blueprints/Widgets/GrenadeMultiplier.MakeProgressbarVisible` (`self.WidgetGrenadeMultiplier`))
  (bind (_direction _newtrack_0) (`Timeline|Timeline_0` :!via `PlayFromStart`)
    (:`Update`
      (bind _output_get (set `self.GrenadeMultiplier` _newtrack_0))
      (`KismetSystemLibrary.PrintString` (`KismetStringLibrary.Conv_DoubleToString` _output_get)))))

(event `self.CallReleaseGrenade`
  (`/Game/Blueprints/Widgets/GrenadeMultiplier.MakeProgressbarInvisible` (`self.WidgetGrenadeMultiplier`))
  (`self.ReleaseGrenade`))

(fn `UserConstructionScript`)