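; BP_DroneCharacter is a drone character with animations for deploying from a backpack.
; Custom events play a timeline that rotates the drone mesh between backpack and deployed rotations, reversing it to stow.
; A separate lift event saves the pre-deploy transform, raises the actor with a swept timeline move, then sets the capsule to overlap pawns.
; Nothing here calls these events, and RotateToDeployedF is an empty stub.
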(event `self.RotateToDeployed`
  (bind (_direction _newtrack_0) (`Timeline|RotateToDeployedTL` :!via `PlayFromStart` :!label _label)
    (:`Update`
      (`SceneComponent.K2_SetRelativeRotation` (`self.DroneMesh`) (`KismetMathLibrary.RLerp` (`self.RotationBackPack`) (`self.RotationDeployed`) _newtrack_0 true) false false))))

(event `self.RotateToBackPack`
  (goto _label :!via `Reverse`))

(event `self.LiftFromBackPack`
  (bind _locationbackpack (`self.LocationBackPack`))
  (set `self.RotationActorBeforeDeploy` (`self.K2_GetActorRotation`))
  (set `self.LocationActorBeforeDeploy` (`self.K2_GetActorLocation`))
  (set `self.LocationBackPack` (`self.K2_GetActorLocation`))
  (bind (_direction _newtrack_0) (`Timeline|Timeline_0` :!via `PlayFromStart`)
    (:`Update`
      (`self.K2_SetActorLocation` (`KismetMathLibrary.VLerp` _locationbackpack (+ _locationbackpack (0.0 0.0 200.0)) _newtrack_0) true))
    (:`Finished`
      (`PrimitiveComponent.SetCollisionResponseToChannel` (`self.CapsuleComponent`) "ECC_Pawn" "ECR_Overlap"))))

(fn `RotateToDeployed_f`)

(fn `UserConstructionScript`)